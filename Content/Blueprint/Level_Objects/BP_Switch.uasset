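; BP_Switch is an interactable level switch that toggles a light in the scene on and off.
; On BeginPlay it binds SwitchStart to the interaction event of its CBPInteractable component.
; Each interaction runs a FlipFlop that tilts the SwitchFlip part to the opposite angle and sets the intensity of LightInScene.
; Disconnected loops over a MyLight array remain in the graph and never run.
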(event `self.ReceiveBeginPlay`
  (add `/Game/Blueprint/Components/CBP_Interactable.ED_Interaction` (`self.CBP_Interactable`) (delegate `SwitchStart`)))

(event `SwitchStart`
  (`/Engine/EditorBlueprintResources/StandardMacros.FlipFlop`
    (:`A`
      (`SceneComponent.K2_SetRelativeRotation` (`self.SwitchFlip`) (struct :`Roll` -30.0) false false)
      (`LightComponent.SetIntensity` (`Light.LightComponent` (`self.LightInScene`)) 20.0))
    (:`B`
      (`SceneComponent.K2_SetRelativeRotation` (`self.SwitchFlip`) (struct :`Roll` 30.0) false false)
      (`LightComponent.SetIntensity` (`Light.LightComponent` (`self.LightInScene`)) 0.0))))

(fn `UserConstructionScript`)